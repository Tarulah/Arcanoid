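; Ball actor for a Breakout-style game on the XZ plane, reflecting its movement velocity off hard-coded side and top bounds checked every Tick.
; Falling below the bottom bound returns it to its BeginPlay position, relaunches it downward and attempts a batch of random BreakableBox spawns, skipping colliding spots, without clearing existing boxes.
; Hitting a tagged box when at most one remains jumps into that same reset-and-spawn loop as the win restart.
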(event `PosXBallBounds`
  ;[1 1 1] Right side bounds for ball
  (`/Engine/EditorBlueprintResources/StandardMacros.CompareFloat` (.x (`SceneComponent.K2_GetComponentLocation` (`self.BallMesh`))) 290.0
    (:`>`
      (set `MovementComponent.Velocity` (`KismetMathLibrary.MakeVector` (* (.x (`MovementComponent.Velocity` (`self.BallMovement`))) -1.0) (.y (`MovementComponent.Velocity` (`self.BallMovement`))) (.z (`MovementComponent.Velocity` (`self.BallMovement`)))) (`self.BallMovement`)))))

(event `NegXBallBounds`
  ;[1 1 1] Left side bounds for ball
  (`/Engine/EditorBlueprintResources/StandardMacros.CompareFloat` (.x (`SceneComponent.K2_GetComponentLocation` (`self.BallMesh`))) -290.0
    (:`<`
      (set `MovementComponent.Velocity` (`KismetMathLibrary.MakeVector` (* (.x (`MovementComponent.Velocity` (`self.BallMovement`))) -1.0) (.y (`MovementComponent.Velocity` (`self.BallMovement`))) (.z (`MovementComponent.Velocity` (`self.BallMovement`)))) (`self.BallMovement`)))))

(event `self.ReceiveBeginPlay`
  ;[1 1 1] Set balls starting position
  (set `self.BallStartPos` (`SceneComponent.K2_GetComponentLocation` (`self.BallMesh`))))

(event `self.ReceiveTick`
  (params (DeltaSeconds :type "Float (single-precision)"))
  (`|ExecutionSequence`
    (:`then_0`
      (`self.PosXBallBounds`))
    (:`then_1`
      (`self.NegXBallBounds`))
    (:`then_2`
      (`self.PosZBallBounds`))
    (:`then_3`
      (`self.NegZBallBounds`))))

(event `PosZBallBounds`
  ;[1 1 1] Upper bounds for ball
  (`/Engine/EditorBlueprintResources/StandardMacros.CompareFloat` (.z (`SceneComponent.K2_GetComponentLocation` (`self.BallMesh`))) 233.0
    (:`>`
      (set `MovementComponent.Velocity` (`KismetMathLibrary.MakeVector` (.x (`MovementComponent.Velocity` (`self.BallMovement`))) (.y (`MovementComponent.Velocity` (`self.BallMovement`))) (* (.z (`MovementComponent.Velocity` (`self.BallMovement`))) -1.0)) (`self.BallMovement`)))))

(event `NegZBallBounds`
  ;[1 1 1] Down bounds for ball
  (`/Engine/EditorBlueprintResources/StandardMacros.CompareFloat` (.z (`SceneComponent.K2_GetComponentLocation` (`self.BallMesh`))) -30.0
    (:`<`
      ;[1 1 1] Restart game if win
      (for _ (range 1 21) :!label _label
        (`|SpawnActorFromClass` "/Game/Blueprints/BreakableBox.BreakableBox_C" (`KismetMathLibrary.MakeTransform` (`KismetMathLibrary.MakeVector` (`KismetMathLibrary.RandomFloatInRange` -250.0 260.0) 0.0 (`KismetMathLibrary.RandomFloatInRange` 40.0 200.0))) "DontSpawnIfColliding" "OverrideRootScale")
        (`self.K2_SetActorLocation` (`self.BallStartPos`))
        (`ProjectileMovementComponent.SetVelocityInLocalSpace` (`self.BallMovement`) (0.0 0.0 -200.0))))))

(event `self.ReceiveHit`
  (params (MyComp :type "PrimitiveComponent Object Reference") (Other :type "Actor Object Reference") (OtherComp :type "PrimitiveComponent Object Reference") (bSelfMoved :type Boolean) (HitLocation :type "Vector Structure") (HitNormal :type "Vector Structure") (NormalImpulse :type "Vector Structure") (Hit :type "HitResult Structure (by ref)"))
  ;[1 1 1] Restart game if win
  (if (`ActorComponent.ComponentHasTag` OtherComp "BoxTag")
    (bind _outactors (`GameplayStatics.GetAllActorsOfClass` "/Game/Blueprints/BreakableBox.BreakableBox_C"))
    (if (not (> (`KismetArrayLibrary.Array_Length` _outactors) 1))
      (goto _label))))

(fn `UserConstructionScript`)