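; PlayerPlatform is a player-controlled platform that slides along the world X axis within fixed limits.
; MoveRight and MoveLeft axis inputs both feed AddMovementInput along positive X, so direction depends on the axis value's sign.
; Every Tick runs two custom bounds events that check the Platform component's world X and use SetActorLocation to snap the actor back to the symmetric limit it crosses.
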(event `InputAxis|MoveRight`
  (params (AxisValue :type "Float (single-precision)"))
  ;[1 1 1] Player movement
  (`self.AddMovementInput` (1.0 0.0 0.0) AxisValue))

(event `GetNegXBouds`
  ;[1 1 1] Check bounds
  (`/Engine/EditorBlueprintResources/StandardMacros.CompareFloat` (.x (`SceneComponent.K2_GetComponentLocation` (`self.Platform`))) -290.0
    (:`<`
      (`self.K2_SetActorLocation` (`KismetMathLibrary.MakeVector` -290.0 (.y (`SceneComponent.K2_GetComponentLocation` (`self.Platform`))) (.z (`SceneComponent.K2_GetComponentLocation` (`self.Platform`))))))))

(event `self.ReceiveTick`
  (params (DeltaSeconds :type "Float (single-precision)"))
  (`|ExecutionSequence`
    (:`then_0`
      (`self.GetNegXBouds`))
    (:`then_1`
      ;[1 1 1] Check bounds
      (`self.GetPosXBounds`))))

(event `InputAxis|MoveLeft`
  (params (AxisValue :type "Float (single-precision)"))
  ;[1 1 1] Player movement
  (`self.AddMovementInput` (1.0 0.0 0.0) AxisValue))

(event `GetPosXBounds`
  ;[1 1 1] Check bounds
  (`/Engine/EditorBlueprintResources/StandardMacros.CompareFloat` (.x (`SceneComponent.K2_GetComponentLocation` (`self.Platform`))) 290.0
    (:`>`
      (`self.K2_SetActorLocation` (`KismetMathLibrary.MakeVector` 290.0 (.y (`SceneComponent.K2_GetComponentLocation` (`self.Platform`))) (.z (`SceneComponent.K2_GetComponentLocation` (`self.Platform`))))))))

(fn `UserConstructionScript`)